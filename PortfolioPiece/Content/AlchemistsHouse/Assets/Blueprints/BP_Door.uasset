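; BP_Door is an interactive double door that the first-person character opens and closes with an on-screen "Press E" prompt.
; A trigger box shows the prompt widget on overlap and sets the door reference and open permission on the character, clearing them on exit.
; OpenDoor uses a FlipFlop to alternately play or reverse a timeline that swings both leaves' yaw in opposite directions while updating the prompt text.
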(event OnComponentBeginOverlap(Box)
  (params (OverlappedComponent :type Primitive%20Component%20Object%20Reference) (OtherActor :type Actor%20Object%20Reference) (OtherComp :type Primitive%20Component%20Object%20Reference) (OtherBodyIndex :type Integer) (bFromSweep :type Boolean) (SweepResult :type Hit%20Result%20Structure%20%28by%20ref%29))
  (bind _asbp_first_person_character (Utilities|Casting|CastToBP_FirstPersonCharacter OtherActor))
  (bind _returnvalue (UserInterface|CreateWidget "/Game/AlchemistsHouse/Assets/Blueprints/UMG_PressToOpen.UMG_PressToOpen_C" 0 (Variables|Default|GetOpenCloseText)))
  (bind _output_get (Variables|Default|SetUI%20Info _returnvalue))
  (UserInterface|Viewport|AddtoViewport _output_get 0)
  (Variables|/Game/FirstPerson/Blueprints/BP_FirstPersonCharacter.BP_FirstPersonCharacter_C|SetCanOpenDoor? _asbp_first_person_character true)
  (Variables|/Game/FirstPerson/Blueprints/BP_FirstPersonCharacter.BP_FirstPersonCharacter_C|SetDoorReference _asbp_first_person_character self))

(event OnComponentEndOverlap(Box)
  (params (OverlappedComponent :type Primitive%20Component%20Object%20Reference) (OtherActor :type Actor%20Object%20Reference) (OtherComp :type Primitive%20Component%20Object%20Reference) (OtherBodyIndex :type Integer))
  (bind _asbp_first_person_character (Utilities|Casting|CastToBP_FirstPersonCharacter OtherActor))
  (Widget|RemovefromParent (Variables|Default|GetUI%20Info))
  (Variables|/Game/FirstPerson/Blueprints/BP_FirstPersonCharacter.BP_FirstPersonCharacter_C|SetCanOpenDoor? _asbp_first_person_character false)
  (Variables|/Game/FirstPerson/Blueprints/BP_FirstPersonCharacter.BP_FirstPersonCharacter_C|SetDoorReference _asbp_first_person_character 0))

(event Custom|OpenDoor
  (bind _door3 (Variables|Default|GetDoor3))
  (bind _door2 (Variables|Default|GetDoor2))
  (bind _ui_info (Variables|Default|GetUI%20Info))
  (bind _returnvalue (Transformation|GetWorldRotation _door3))
  (bind _returnvalue_2 (Transformation|GetWorldRotation _door2))
  (Utilities|FlowControl|FlipFlop
    (:A
      (bind _output_get (Variables|Default|SetOpenCloseText "Press E to Close"))
      (Default|UpdateText _ui_info _output_get)
      (bind _openingdoors (Timeline|OpenDoors PlayFromStart)
        (:Update
          (Transformation|SetRelativeRotation _door2 (Math|Rotator|MakeRotator (.roll _returnvalue_2) (.pitch _returnvalue_2) (Math|Float|Lerp 0.0 -9e+01 _openingdoors)) false false)
          (Transformation|SetRelativeRotation _door3 (Math|Rotator|MakeRotator (.roll _returnvalue) (.pitch _returnvalue) (Math|Float|Lerp 1.8e+02 2.7e+02 _openingdoors)) false false))))
    (:B
      (bind _output_get_2 (Variables|Default|SetOpenCloseText "Press E to Open"))
      (Default|UpdateText _ui_info _output_get_2)
      (Timeline|OpenDoors Reverse))))

(fn ConstructionScript)